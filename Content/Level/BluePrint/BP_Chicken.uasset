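; BP_Chicken is a collectable pickup that spins and bobs in the level.
; Each Tick adds a fixed yaw step to the mesh and offsets the actor vertically by the sine of an accumulating angle.
; When something overlaps PickUpRadius, its instigator is cast to BP_ThirdPersonCharacter.
; On success, that character's Chicken count increments and prints, and the pickup destroys itself.
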(event `self.Pick Up Radius.OnComponentBeginOverlap`
  (params (OverlappedComponent :type "PrimitiveComponent Object Reference") (OtherActor :type "Actor Object Reference") (OtherComp :type "PrimitiveComponent Object Reference") (OtherBodyIndex :type Integer) (bFromSweep :type Boolean) (SweepResult :type "HitResult Structure (by ref)"))
  (`self.Collectable Chicken` OtherActor))

(event `self.ReceiveTick`
  (params (DeltaSeconds :type "Float (single-precision)"))
  (`|ExecutionSequence`
    (:`then_0`
      (`self.Rotation`))
    (:`then_1`
      (`self.Up&down` DeltaSeconds))))

(fn `Collectable Chicken`
  (params (self2 :type "Actor Object Reference"))
  (bind _asbp_third_person_character (cast `/Game/ThirdPerson/Blueprints/BP_ThirdPersonCharacter` (`self.GetInstigator` self2)))
  (bind _result (`/Engine/EditorBlueprintResources/StandardMacros.IncrementInt` (`/Game/ThirdPerson/Blueprints/BP_ThirdPersonCharacter.Chicken` _asbp_third_person_character))
    (:`  `
      (`KismetSystemLibrary.PrintString` (`KismetStringLibrary.Conv_IntToString` _result))
      (`self.K2_DestroyActor`))))

(fn `Rotation`
  (`SceneComponent.K2_AddRelativeRotation` (`self.Mesh`) (`KismetMathLibrary.MakeRotator` 0.0 0.0 1.0) false false))

(fn `Up&down`
  (params (A :type "Float (double-precision)"))
  (bind _output_get (set `self.sin degress` (+ (* A 100.0) (`self.sin degress`))))
  (`self.K2_AddActorWorldOffset` (`KismetMathLibrary.MakeVector` 0.0 0.0 (`KismetMathLibrary.DegSin` _output_get))))

(fn `UserConstructionScript`)